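; BP_P38 is a player-controlled plane pawn that constantly flies forward along its forward vector every tick.
; On begin play it registers the Propeller with BPRotateComponent so that the component spins it.
; Enhanced Input drives frame-rate-scaled local roll and pitch through IA_PitchNRoll, and IA_Fire spawns a BP_Rocket at the Arrow component's transform.
; The construction script and RotatePropeller function are empty.
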(event `self.ReceiveTick`
  (params (DeltaSeconds :type "Float (single-precision)"))
  ;[1 1 1] 전진
  (`self.AddMovementInput` (`self.GetActorForwardVector`)))

(event `self.ReceiveBeginPlay`
  ;[1 1 1] 시작하면 물체회전
  (`/Game/BP/BP_RotateComponent.AddSceneComp` (`self.BP_RotateComponent`) (`self.Propeller`)))

(event `EnhancedInput|/Game/Input/IA_PitchNRoll`
  (params (ActionValue :type "Vector2D Structure") (ElapsedSeconds :type "Float (double-precision)") (TriggeredSeconds :type "Float (double-precision)") (InputAction :type "InputAction Object Reference" :default "/Game/Input/IA_PitchNRoll.IA_PitchNRoll"))
  ;[1 1 1] Enhanced Input  을 이용한 Pitch Roll 제어
  (:`Triggered`
    (`self.K2_AddActorLocalRotation` (`KismetMathLibrary.MakeRotator` (* ActionValue_X (`GameplayStatics.GetWorldDeltaSeconds`) 60.0)))
    (`self.K2_AddActorLocalRotation` (`KismetMathLibrary.MakeRotator` 0.0 (* ActionValue_Y (`GameplayStatics.GetWorldDeltaSeconds`) 60.0)))))

(event `EnhancedInput|/Game/Input/IA_Fire`
  (params (ActionValue :type Boolean) (ElapsedSeconds :type "Float (double-precision)") (TriggeredSeconds :type "Float (double-precision)") (InputAction :type "InputAction Object Reference" :default "/Game/Input/IA_Fire.IA_Fire"))
  (:`Triggered`
    (`|SpawnActorFromClass` "/Game/BP/BP_Rocket.BP_Rocket_C" (`SceneComponent.K2_GetComponentToWorld` (`self.Arrow`)) "Undefined" "MultiplyWithRoot" null null)))

(fn `RotatePropeller`)

(fn `UserConstructionScript`)